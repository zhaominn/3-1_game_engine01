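; BP_AutoFence is an actor that procedurally builds a fence from its origin to the FenceEnd point.
; The construction script derives direction and rotation from FenceEnd, then adds static mesh panels at fixed intervals along that line.
; Each panel gets slight random yaw and height scale variation to break up repetition.
; The event graph holds only disabled placeholder events, so it has no gameplay logic.
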(event EventBeginPlay)

(event Collision|EventActorBeginOverlap
  (params (OtherActor :type Actor%20Object%20Reference)))

(event EventTick
  (params (DeltaSeconds :type Float%20%28single-precision%29)))

(fn ConstructionScript
  (bind _fence_end (Variables|Default|GetFence%20End))
  (bind _output_get (Variables|Default|SetFence%20Growing%20Direction (Math|Vector|GetUnitDirection(Vector) "0, 0, 0" _fence_end)))
  (Variables|Default|SetPanel%20Rotation (Math|Conversions|RotationFromXVector _output_get))
  (for _index (range 0 (Math|Float|Truncate (/ (Math|Vector|VectorLength _fence_end) 2e+01)))
    (AddComponent|AddStaticMeshComponent false (Math|Transform|MakeTransform (* _index 2e+01 (Variables|Default|GetFence%20Growing%20Direction)) (Math|Rotator|CombineRotators (Variables|Default|GetPanel%20Rotation) (Math|Rotator|MakeRotator 0.0 0.0 (Math|Random|RandomFloatinRange -5.0 5.0))) (Math|Vector|MakeVector 1.0 0.0 (Math|Random|RandomFloatinRange 1.0 1.02))))))