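; Player controller for an aircraft pawn that turns Enhanced Input actions into look and movement input.
; On BeginPlay it registers the aircraft control mapping context with the local player's input subsystem.
; The rotate action feeds yaw and pitch to the controller.
; The translate action moves the controlled pawn along its own forward and right vectors.
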(event Input|EnhancedActionEvents|EnhancedInputActionIA_RotateAircraft
  (params (ActionValue :type Vector%202D%20Structure) (ElapsedSeconds :type Float%20%28double-precision%29) (TriggeredSeconds :type Float%20%28double-precision%29) (InputAction :type Input%20Action%20Object%20Reference :default "/Game/LEC08_InputSystem/IA_RotateAircraft.IA_RotateAircraft"))
  (Class|PlayerController|AddYawInput (.x ActionValue))
  (Class|PlayerController|AddPitchInput (.y ActionValue)))

(event Input|EnhancedActionEvents|EnhancedInputActionIA_TranslateAircraft
  (params (ActionValue :type Vector%202D%20Structure) (ElapsedSeconds :type Float%20%28double-precision%29) (TriggeredSeconds :type Float%20%28double-precision%29) (InputAction :type Input%20Action%20Object%20Reference :default "/Game/LEC08_InputSystem/IA_TranslateAircraft.IA_TranslateAircraft"))
  (bind _returnvalue (Pawn|GetControlledPawn))
  (Pawn|Input|AddMovementInput _returnvalue (Transformation|GetActorForwardVector _returnvalue) (.x ActionValue) false)
  (Pawn|Input|AddMovementInput _returnvalue (Transformation|GetActorRightVector _returnvalue) (.y ActionValue) false))

(event EventBeginPlay
  (Input|AddMappingContext (PlayerController|LocalPlayerSubsystems|GetEnhancedInputLocalPlayerSubsystem) "/Game/LEC08_InputSystem/IMC_AircraftControl.IMC_AircraftControl" 0 "(bIgnoreAllPressedKeysUntilRelease=True,bForceImmediately=False,bNotifyUserSettings=False)"))

(event EventTick
  (params (DeltaSeconds :type Float%20%28single-precision%29)))

(fn ConstructionScript)