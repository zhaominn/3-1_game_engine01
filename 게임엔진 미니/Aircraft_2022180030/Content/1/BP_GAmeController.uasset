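; BP_GAmeController is a player controller that handles movement and look input, HUD creation and music.
; On BeginPlay it adds the IMC_Control Enhanced Input mapping context, puts BP_Widget on the viewport and plays a 2D music track.
; IA_Rotater feeds yaw and pitch input to the controller.
; IA_Translate moves the controlled pawn along its own forward and right vectors.
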(event Input|EnhancedActionEvents|EnhancedInputActionIA_Rotater
  (params (ActionValue :type Vector%202D%20Structure) (ElapsedSeconds :type Float%20%28double-precision%29) (TriggeredSeconds :type Float%20%28double-precision%29) (InputAction :type Input%20Action%20Object%20Reference :default "/Game/1/IA_Rotater.IA_Rotater"))
  (Class|PlayerController|AddYawInput (.x ActionValue))
  (Class|PlayerController|AddPitchInput (.y ActionValue)))

(event Input|EnhancedActionEvents|EnhancedInputActionIA_Translate
  (params (ActionValue :type Vector%202D%20Structure) (ElapsedSeconds :type Float%20%28double-precision%29) (TriggeredSeconds :type Float%20%28double-precision%29) (InputAction :type Input%20Action%20Object%20Reference :default "/Game/1/IA_Translate.IA_Translate"))
  (bind _returnvalue (Pawn|GetControlledPawn))
  (Pawn|Input|AddMovementInput _returnvalue (Transformation|GetActorForwardVector _returnvalue) (.x ActionValue) false)
  (Pawn|Input|AddMovementInput _returnvalue (Transformation|GetActorRightVector _returnvalue) (.y ActionValue) false))

(event EventBeginPlay
  (Input|AddMappingContext (PlayerController|LocalPlayerSubsystems|GetEnhancedInputLocalPlayerSubsystem) "/Game/1/IMC_Control.IMC_Control" 0 "(bIgnoreAllPressedKeysUntilRelease=True,bForceImmediately=False,bNotifyUserSettings=False)")
  (bind _returnvalue (UserInterface|CreateWidget "/Game/1/BP_Widget.BP_Widget_C"))
  (UserInterface|Viewport|AddtoViewport _returnvalue 0)
  (Audio|PlaySound2D "/Game/Easy_Listening_BGM_Vol_1/14__Soulful_Upbeat_Melody_and_Horn.14__Soulful_Upbeat_Melody_and_Horn" 1.0 1.0 0.0 0 0))

(event EventTick
  (params (DeltaSeconds :type Float%20%28single-precision%29)))

(fn ConstructionScript)