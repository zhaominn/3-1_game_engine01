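; BP_Aircraft is an aircraft actor that drops bombs on input and tracks its distance from where it started.
; The IA_Bomb action spawns a BP_Bomb at BombPoint with an explosion sound and particle effect.
; Each tick updates the straight-line distance, records game time as elapsed time until the ENd flag is set, and spawns a new steam emitter at BombPoint.
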(event Input|EnhancedActionEvents|EnhancedInputActionIA_Bomb
  (params (ActionValue :type Boolean) (ElapsedSeconds :type Float%20%28double-precision%29) (TriggeredSeconds :type Float%20%28double-precision%29) (InputAction :type Input%20Action%20Object%20Reference :default "/Game/1/IA_Bomb.IA_Bomb"))
  (bind _bomb_point (Variables|Default|Getbomb%20point))
  (bind _returnvalue (Transformation|GetWorldLocation _bomb_point))
  (:Started
    (Game|SpawnActorfromClass "/Game/1/BP_Bomb.BP_Bomb_C" (Math|Conversions|ToTransform(Vector) _returnvalue) "AlwaysSpawn" "MultiplyWithRoot" 0 0)
    (Audio|PlaySoundatLocation "/Game/StarterContent/Audio/Explosion02.Explosion02" _returnvalue "0, 0, 0" 1.0 1.0 0.0 0 0 0 0)
    (Effects|SpawnEmitteratLocation "/Game/StarterContent/Particles/P_Explosion.P_Explosion" _returnvalue)))

(event EventBeginPlay
  (Variables|Default|Setstart%20location (Transformation|GetActorLocation)))

(event Collision|EventActorBeginOverlap
  (params (OtherActor :type Actor%20Object%20Reference)))

(event EventTick
  (params (DeltaSeconds :type Float%20%28single-precision%29))
  (CallFunction|UpdateTime)
  (Variables|Default|Setplayer%20distance (Math|Vector|Distance(Vector) (Transformation|GetActorLocation) (Variables|Default|Getstart%20location)))
  (Effects|SpawnEmitteratLocation "/Game/StarterContent/Particles/P_Steam_Lit.P_Steam_Lit" (Transformation|GetWorldLocation (Variables|Default|Getbomb%20point)) "0, 0, 0" "0.500000,0.500000,0.500000"))

(fn ConstructionScript)

(fn UpdateTime
  (if (not (Variables|Default|GetENd?))
    (Variables|Default|Setelapsed%20time (Utilities|Time|GetTimeSeconds))))