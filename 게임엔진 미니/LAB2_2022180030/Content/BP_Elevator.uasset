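; BP_Elevator is an elevator actor that rises while something overlaps its Box trigger and otherwise runs its FloatingComponent.
; Box overlap start sets OnBoard and turns floating off, and Tick then adds a fixed, frame-rate-dependent upward offset.
; Overlap end clears OnBoard, turns floating back on and sets its BaseLocation to the current position, with no descent logic or actor filter.
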(event OnComponentBeginOverlap(Box)
  (params (OverlappedComponent :type Primitive%20Component%20Object%20Reference) (OtherActor :type Actor%20Object%20Reference) (OtherComp :type Primitive%20Component%20Object%20Reference) (OtherBodyIndex :type Integer) (bFromSweep :type Boolean) (SweepResult :type Hit%20Result%20Structure%20%28by%20ref%29))
  (Development|PrintText "Enter")
  (Variables|Default|SetOn%20Board? true)
  (Default|TurnOff (Variables|Default|GetFloatingComponent)))

(event OnComponentEndOverlap(Box)
  (params (OverlappedComponent :type Primitive%20Component%20Object%20Reference) (OtherActor :type Actor%20Object%20Reference) (OtherComp :type Primitive%20Component%20Object%20Reference) (OtherBodyIndex :type Integer))
  (bind _floatingcomponent (Variables|Default|GetFloatingComponent))
  (Development|PrintText "Leave")
  (Variables|Default|SetOn%20Board? false)
  (Default|Turnon _floatingcomponent)
  (Variables|/Game/FloatingComponent.FloatingComponent_C|SetBase%20Location _floatingcomponent (Transformation|GetActorLocation)))

(event EventBeginPlay
  (Default|Turnon (Variables|Default|GetFloatingComponent)))

(event Collision|EventActorBeginOverlap
  (params (OtherActor :type Actor%20Object%20Reference)))

(event EventTick
  (params (DeltaSeconds :type Float%20%28single-precision%29))
  (if (Variables|Default|GetOn%20Board?)
    (Transformation|AddActorLocalOffset (Math|Vector|MakeVector 0.0 0.0 1.0) false false)))

(fn ConstructionScript)